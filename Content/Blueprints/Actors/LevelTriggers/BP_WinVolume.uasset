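; BP_WinVolume is a level trigger that decides the outcome when the player overlaps it.
; If any BP_Crystal actors remain in the world it quits the game, otherwise it completes the level.
; Completion finds the current level in the LevelNames array and opens the next entry by name.
; On the final level in that array, completion does nothing.
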(event Collision|EventActorBeginOverlap
  (params (OtherActor :type Actor%20Object%20Reference))
  (Utilities|IsPlayer OtherActor
    (:IsPlayer
      (if (LevelManagement|AnyCrystalsRemaining)
        (Game|QuitGame 0 "Quit" false)
        (else
          (LevelManagement|CompleteLevel))))))

(fn ConstructionScript)

(fn AnyCrystalsRemaining
  (bind _outactors (Actor|GetAllActorsOfClass "/Game/Blueprints/Actors/Collectibles/BP_Crystal.BP_Crystal_C"))
  (return (> (Utilities|Array|Length _outactors) 0)))

(fn GetCurrentLevelIndex
  (bind _returnvalue (Game|GetCurrentLevelName true))
  (return (Utilities|Array|FindItem (Variables|Default|GetLevel%20Names) (Utilities|String|StringToName _returnvalue))))

(fn CompleteLevel
  (if (not (LevelManagement|IsFinalLevel))
    (LevelManagement|LoadNextLevel)))

(fn IsFinalLevel
  (return (== (Utilities|Array|LastIndex (Variables|Default|GetLevel%20Names)) (LevelManagement|GetCurrentLevelIndex))))

(fn LoadNextLevel
  (Game|OpenLevel(byName) (CallFunction|GetNextLevelName)))

(fn GetNextLevelName
  (return (Utilities|Array|Get(acopy) (Variables|Default|GetLevel%20Names) (+ (LevelManagement|GetCurrentLevelIndex) 1))))